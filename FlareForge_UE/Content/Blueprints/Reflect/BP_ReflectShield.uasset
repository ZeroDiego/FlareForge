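; BP_ReflectShield is a timed shield actor that deflects other players' projectiles and destroys itself after ActiveTimer.
; Its box overlap sets collision to Ignore for basic or homing projectiles owned by the stored player reference.
; For others, the server spawns a same-class projectile behind the incoming one, facing backward and owned by the shield's player.
; Reflected homing projectiles immediately lock onto a newly found target.
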(event `self.ReceiveBeginPlay`
  (`KismetSystemLibrary.Delay` (`self.ActiveTimer`))
  (`self.K2_DestroyActor`))

(event `self.GetDeflectPlayerReference`
  (params (PlayerSpawningRootComponent :type "SceneComponent Object Reference"))
  (`self.RPC Get Deflect Player Reference` PlayerSpawningRootComponent))

(event `RPC Get Deflect Player Reference`
  (params (PlayerShieldReference :type "SceneComponent Object Reference"))
  (set `self.PlayerRef` PlayerShieldReference))

(event `self.BoxComponent.OnComponentBeginOverlap`
  (params (OverlappedComponent :type "PrimitiveComponent Object Reference") (OtherActor :type "Actor Object Reference") (OtherComp :type "PrimitiveComponent Object Reference") (OtherBodyIndex :type Integer) (bFromSweep :type Boolean) (SweepResult :type "HitResult Structure (by ref)"))
  (bind _returnvalue (* (`self.GetActorForwardVector` OtherActor) -100.0))
  (bind _returnvalue_location (`KismetMathLibrary.BreakTransform` (`KismetMathLibrary.Conv_VectorToTransform` (+ _returnvalue (`self.K2_GetActorLocation` OtherActor)))))
  (`|ExecutionSequence`
    (:`then_0`
      (bind _asbp_basic_projecitle (cast `/Game/Blueprints/Projectiles/BP_BasicProjecitle` OtherActor)
        (:`then`
          (if (== (`self.PlayerRef`) (`/Game/Blueprints/Projectiles/BP_BasicProjecitle.PlayerRootComponent` _asbp_basic_projecitle))
            (`PrimitiveComponent.SetCollisionResponseToChannel` (`/Game/Blueprints/Projectiles/BP_BasicProjecitle.TriggerBox` _asbp_basic_projecitle) "ECC_GameTraceChannel3" "ECR_Ignore")
            (else
              (if (`self.HasAuthority`) :!label _label
                (bind _returnvalue_2 (`|SpawnActorFromClass` (`GameplayStatics.GetObjectClass` OtherActor) (`KismetMathLibrary.MakeTransform` _returnvalue_location (`KismetMathLibrary.Conv_VectorToRotator` _returnvalue)) "AdjustIfPossibleButAlwaysSpawn" "MultiplyWithRoot" null null))
                (bind _asbp_basic_projecitle_2 (cast `/Game/Blueprints/Projectiles/BP_BasicProjecitle` _returnvalue_2)
                  (:`then`
                    (`/Engine/EditorBlueprintResources/StandardMacros.IsValid` _asbp_basic_projecitle_2
                      (:`Is Valid`
                        (set `/Game/Blueprints/Projectiles/BP_BasicProjecitle.PlayerRootComponent` (`self.PlayerRef`) _asbp_basic_projecitle_2))))
                  (:`CastFailed`
                    (bind _asbp_homing_strike_projectile (cast `/Game/Blueprints/Projectiles/BP_HomingStrikeProjectile` _returnvalue_2))
                    (`/Engine/EditorBlueprintResources/StandardMacros.IsValid` _asbp_homing_strike_projectile
                      (:`Is Valid`
                        (bind _output_get (set `/Game/Blueprints/Projectiles/BP_HomingStrikeProjectile.PlayerSpawningReference` (`self.PlayerRef`) _asbp_homing_strike_projectile))
                        (`HomingStrikeProjectile.LockOn` _asbp_homing_strike_projectile (`HomingStrikeProjectile.FindHomingStrikeTarget` _asbp_homing_strike_projectile) _output_get)))))))))
        (:`CastFailed`
          (bind _asbp_homing_strike_projectile_2 (cast `/Game/Blueprints/Projectiles/BP_HomingStrikeProjectile` OtherActor))
          (if (== (`self.PlayerRef`) (`/Game/Blueprints/Projectiles/BP_HomingStrikeProjectile.PlayerSpawningReference` _asbp_homing_strike_projectile_2))
            (`PrimitiveComponent.SetCollisionResponseToChannel` (`/Game/Blueprints/Projectiles/BP_HomingStrikeProjectile.TriggerBox` _asbp_homing_strike_projectile_2) "ECC_GameTraceChannel3" "ECR_Ignore")
            (else
              (goto _label))))))
    (:`then_1`
      (goto _label_2 :!via `Reset`))))

(event `self.BoxComponent.OnComponentEndOverlap`
  (params (OverlappedComponent :type "PrimitiveComponent Object Reference") (OtherActor :type "Actor Object Reference") (OtherComp :type "PrimitiveComponent Object Reference") (OtherBodyIndex :type Integer))
  (`/Engine/EditorBlueprintResources/StandardMacros.DoOnce` false :!label _label_2
    (:`Completed`
      (bind _asbp_basic_projecitle (cast `/Game/Blueprints/Projectiles/BP_BasicProjecitle` OtherActor))
      (`PrimitiveComponent.SetCollisionResponseToChannel` (`/Game/Blueprints/Projectiles/BP_BasicProjecitle.TriggerBox` _asbp_basic_projecitle) "ECC_GameTraceChannel3" "ECR_Overlap"))))

(fn `UserConstructionScript`)