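; Respawning center health pickup that appears with a spawn sound after a short delay at BeginPlay.
; Overlap by a BP_MyPlayerCharacter while visible calls that character's CenterHealthPickupOnServer, plays a pickup sound and hides the capsule, then re-shows it after a delay.
; The NewHidden flag doubles as visibility state and overlap gate.
; Tick uses a game-time sine to bob the capsule and oscillate its yaw.
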(event `self.ReceiveBeginPlay`
  (bind _output_get (set `self.New Hidden` true))
  (`SceneComponent.SetHiddenInGame` (`self.Capsule`) _output_get true)
  (`KismetSystemLibrary.Delay` 1.0)
  (`GameplayStatics.SpawnSoundAtLocation` "/Game/Audio/PickupSounds/spawn_healthpickup.spawn_healthpickup" (`SceneComponent.K2_GetComponentLocation` (`self.Capsule`)) (struct) 1.0 (`KismetMathLibrary.RandomFloatInRange` 0.95 1.1) 0.0 "/Game/Audio/SoundAttenuation/SA_SpawnHealthPickup.SA_SpawnHealthPickup" null)
  (bind _output_get_2 (set `self.New Hidden` false))
  (`SceneComponent.SetHiddenInGame` (`self.Capsule`) _output_get_2 true))

(event `self.ReceiveTick`
  (params (DeltaSeconds :type "Float (single-precision)"))
  (bind _returnvalue (* (* (`KismetMathLibrary.DegSin` (* (`KismetSystemLibrary.GetGameTimeInSeconds`) 100.0)) 0.002) 100.0))
  (`SceneComponent.K2_AddWorldOffset` (`self.Capsule`) (`KismetMathLibrary.MakeVector` 0.0 0.0 _returnvalue) true true)
  (`SceneComponent.K2_AddWorldRotation` (`self.Capsule`) (`KismetMathLibrary.MakeRotator` 0.0 0.0 _returnvalue) false false))

(event `self.Capsule.OnComponentBeginOverlap`
  (params (OverlappedComponent :type "PrimitiveComponent Object Reference") (OtherActor :type "Actor Object Reference") (OtherComp :type "PrimitiveComponent Object Reference") (OtherBodyIndex :type Integer) (bFromSweep :type Boolean) (SweepResult :type "HitResult Structure (by ref)"))
  (bind _capsule (`self.Capsule`))
  (bind _asbp_my_player_character (cast `/Game/TopDown/Blueprints/BP_MyPlayerCharacter` OtherActor))
  (if (not (`self.New Hidden`))
    (`/Game/TopDown/Blueprints/BP_MyPlayerCharacter.CenterHealthPickup_OnServer` _asbp_my_player_character)
    (`GameplayStatics.SpawnSoundAtLocation` "/Game/Audio/PickupSounds/health-pickup.health-pickup" (`SceneComponent.K2_GetComponentLocation` (`self.Capsule`)) (struct) 0.8 (`KismetMathLibrary.RandomFloatInRange` 1.0 1.2) 0.0 null null)
    (bind _output_get (set `self.New Hidden` true))
    (`SceneComponent.SetHiddenInGame` _capsule _output_get true)
    (`KismetSystemLibrary.Delay` 3.0)
    (`GameplayStatics.SpawnSoundAtLocation` "/Game/Audio/PickupSounds/spawn_healthpickup.spawn_healthpickup" (`SceneComponent.K2_GetComponentLocation` (`self.Capsule`)) (struct) 1.0 (`KismetMathLibrary.RandomFloatInRange` 0.95 1.1) 0.0 "/Game/Audio/SoundAttenuation/SA_SpawnHealthPickup.SA_SpawnHealthPickup" null)
    (bind _output_get_2 (set `self.New Hidden` false))
    (`SceneComponent.SetHiddenInGame` _capsule _output_get_2 true)))

(fn `UserConstructionScript`)