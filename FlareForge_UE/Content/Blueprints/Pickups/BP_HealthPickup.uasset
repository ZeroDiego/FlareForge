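; Health pickup that respawns on randomized timers and bobs vertically through a jittered, time-based sine offset applied to its capsule every Tick.
; It starts hidden and appears after a random delay.
; When BP_MyPlayerCharacter overlaps it while visible, it calls that character's HealthPickupOnServer, hides, then reappears after another random delay.
; The NewHidden flag gates pickup, as hiding leaves collision active.
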(event `self.ReceiveTick`
  (params (DeltaSeconds :type "Float (single-precision)"))
  (`SceneComponent.K2_AddWorldOffset` (`self.Capsule`) (`KismetMathLibrary.MakeVector` 0.0 0.0 (* (* (`KismetMathLibrary.DegSin` (* (`KismetSystemLibrary.GetGameTimeInSeconds`) 100.0)) (`KismetMathLibrary.RandomFloatInRange` 0.001 0.002)) 100.0)) true true))

(event `self.ReceiveBeginPlay`
  (bind _capsule (`self.Capsule`))
  (bind _output_get (set `self.New Hidden` true))
  (`SceneComponent.SetHiddenInGame` _capsule _output_get true)
  (`KismetSystemLibrary.Delay` (`KismetMathLibrary.RandomFloatInRange` 10.0 100.0))
  (bind _output_get_2 (set `self.New Hidden` false))
  (`SceneComponent.SetHiddenInGame` _capsule _output_get_2 true))

(event `self.Capsule.OnComponentBeginOverlap`
  (params (OverlappedComponent :type "PrimitiveComponent Object Reference") (OtherActor :type "Actor Object Reference") (OtherComp :type "PrimitiveComponent Object Reference") (OtherBodyIndex :type Integer) (bFromSweep :type Boolean) (SweepResult :type "HitResult Structure (by ref)"))
  (bind _capsule (`self.Capsule`))
  (bind _asbp_my_player_character (cast `/Game/TopDown/Blueprints/BP_MyPlayerCharacter` OtherActor))
  (if (not (`self.New Hidden`))
    (`/Game/TopDown/Blueprints/BP_MyPlayerCharacter.HealthPickup_OnServer` _asbp_my_player_character)
    (bind _output_get (set `self.New Hidden` true))
    (`SceneComponent.SetHiddenInGame` _capsule _output_get true)
    (`KismetSystemLibrary.Delay` (`KismetMathLibrary.RandomFloatInRange` 20.0 60.0))
    (bind _output_get_2 (set `self.New Hidden` false))
    (`SceneComponent.SetHiddenInGame` _capsule _output_get_2 true)))

(fn `UserConstructionScript`)