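; BP_HomingStrikeTarget is an actor that jumps back and forth between two points, apparently as a moving target for a homing strike.
; On BeginPlay it derives LeftPoint and RightPoint by subtracting and adding AmountToMove to its starting location.
; An endless Delay-driven loop then sets its location to each point in turn every three seconds, with no sweep or interpolation.
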(event `self.ReceiveBeginPlay`
  (bind _returnvalue (`self.K2_GetActorLocation`))
  (bind _amounttomove (`self.AmountToMove`))
  (set `self.LeftPoint` (- _returnvalue _amounttomove))
  (set `self.RightPoint` (+ _returnvalue _amounttomove))
  (`self.K2_SetActorLocation` (`self.LeftPoint`) :!label _label)
  (`KismetSystemLibrary.Delay` 3.0)
  (`self.K2_SetActorLocation` (`self.RightPoint`))
  (`KismetSystemLibrary.Delay` 3.0)
  (goto _label))

(fn `UserConstructionScript`)