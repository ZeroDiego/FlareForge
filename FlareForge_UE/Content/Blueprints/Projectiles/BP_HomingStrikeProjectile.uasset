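; Homing projectile that locks onto a target, knocks back and damages the player character it hits, and expires after a set lifetime.
; A lock-on RPC sets the homing target, skipping the spawning player, then repeatedly searches for a new target after a delay.
; Tick polls the trigger box, ignores the spawner, launches the hit character, and applies GAS stun and damage effects.
; It triggers death through the server when the checked attribute reaches zero.
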(event `self.ReceiveBeginPlay`
  (`KismetSystemLibrary.Delay` (`self.LifeSpanTime`))
  (`self.K2_DestroyActor`))

(event `RPC_LockOn`
  (params (TargetComponent :type "SceneComponent Object Reference (by ref)") (PlayerSpawningRootComponent :type "SceneComponent Object Reference (by ref)"))
  (bind _projectilemovement (`self.ProjectileMovement`))
  (set `self.PlayerSpawningReference` PlayerSpawningRootComponent)
  (if (not (== TargetComponent PlayerSpawningRootComponent))
    (set `ProjectileMovementComponent.HomingTargetComponent` TargetComponent _projectilemovement)
    (set `ProjectileMovementComponent.bIsHomingProjectile` true _projectilemovement))
  (`KismetSystemLibrary.Delay` (`self.TargetSwitchTime`))
  (`self.RPC_LockOn` (`self.FindHomingStrikeTarget`) PlayerSpawningRootComponent))

(event `self.LockOn`
  (params (TargetComponent :type "SceneComponent Object Reference") (PlayerSpawningRootComponent :type "SceneComponent Object Reference"))
  (`self.RPC_LockOn` TargetComponent PlayerSpawningRootComponent))

(event `self.ReceiveTick`
  (params (DeltaSeconds :type "Float (single-precision)"))
  (bind _playerspawningreference (`self.PlayerSpawningReference`))
  (bind _overlappingactors (`PrimitiveComponent.GetOverlappingActors` (`self.TriggerBox`) null))
  (bind _output (`|GetArrayItem` _overlappingactors))
  (bind _rootcomponent (`Actor.RootComponent` _output))
  (bind _returnvalue (`KismetMathLibrary.FindLookAtRotation` (`SceneComponent.K2_GetComponentLocation` (`self.DefaultSceneRoot`)) (`SceneComponent.K2_GetComponentLocation` _rootcomponent)))
  (bind (_returnvalue_x _returnvalue_y) (`KismetMathLibrary.BreakVector` (* (`KismetMathLibrary.GetForwardVector` _returnvalue) (`self.KnockbackPower`))))
  (if (`KismetArrayLibrary.Array_IsEmpty` _overlappingactors)
    _
    (elif (`KismetSystemLibrary.IsValid` _output)
      (if (`KismetSystemLibrary.IsValid` _playerspawningreference)
        (if (not (== _rootcomponent _playerspawningreference))
          (bind _asbp_my_player_character (cast `/Game/TopDown/Blueprints/BP_MyPlayerCharacter` _output :!label _label)
            (:`then`
              (`self.K2_SetActorRotation` _returnvalue)
              (`Character.LaunchCharacter` _asbp_my_player_character (`KismetMathLibrary.MakeVector` _returnvalue_x _returnvalue_y) true true)
              (bind _returnvalue_2 (`AbilitySystemBlueprintLibrary.GetAbilitySystemComponent` _asbp_my_player_character))
              (`AbilitySystemComponent.BP_ApplyGameplayEffectToSelf` :`self` _returnvalue_2 :`GameplayEffectClass` "/Game/Blueprints/GameplayEffects/Stuns/GE_BasicProjectileHitStun.GE_BasicProjectileHitStun_C")
              (`AbilitySystemComponent.BP_ApplyGameplayEffectToSelf` :`self` _returnvalue_2 :`GameplayEffectClass` "/Game/Blueprints/GameplayEffects/Damage/GE_HomingProjectileDamage.GE_HomingProjectileDamage_C")
              (bind (_bsuccessfullyfoundattribute _returnvalue_3) (`AbilitySystemBlueprintLibrary.GetFloatAttributeFromAbilitySystemComponent` _returnvalue_2 (struct :`AttributeName` "Health" :`Attribute` "/Script/FlareForge.MyCharacterAttributeSet:Health" :`AttributeOwner` "/Script/CoreUObject.Class'/Script/FlareForge.MyCharacterAttributeSet'")))
              (if _bsuccessfullyfoundattribute
                (if (<= _returnvalue_3 0.0)
                  (`self.PlayerDeath_OnServer`)
                  (else
                    (`self.K2_DestroyActor`)))
                (else
                  (`self.K2_DestroyActor`))))
            (:`CastFailed`
              (`self.K2_DestroyActor`))))
        (else
          (goto _label))))))

(event `PlayerDeath_OnServer`
  (`/Game/TopDown/Blueprints/BP_MyPlayerCharacter.OnDeath_Multicast` (stale `self.ReceiveTick` _asbp_my_player_character)))

(fn `UserConstructionScript`)