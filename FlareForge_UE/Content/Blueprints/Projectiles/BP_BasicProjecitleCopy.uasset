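; Projectile actor that knocks back player characters it overlaps, self-destructing on contact or after its lifespan.
; BeginPlay enables trigger overlap on a custom channel after a short delay.
; Tick polls the first overlapping actor, skipping the spawner via a root component passed through an RPC event.
; A BP_MyPlayerCharacter gets launched horizontally away from the projectile and notified through OnHitOnServer; other actors just destroy it.
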(event `self.ReceiveBeginPlay`
  (`|ExecutionSequence`
    (:`then_0`
      (`KismetSystemLibrary.Delay` 0.1)
      (`PrimitiveComponent.SetCollisionResponseToChannel` (`self.TriggerBox`) "ECC_GameTraceChannel3" "ECR_Overlap"))
    (:`then_1`
      (`KismetSystemLibrary.Delay` (`self.LifeSpanTime`))
      (`self.K2_DestroyActor`))))

(event `RPC_PlayerRootComponent`
  (params (RootComponent :type "SceneComponent Object Reference (by ref)"))
  (set `self.PlayerRootComponent` RootComponent))

(event `self.PlayerSpawningRootComponent`
  (params (PlayerSpawningComponent :type "SceneComponent Object Reference"))
  (`self.RPC_PlayerRootComponent` PlayerSpawningComponent))

(event `self.ReceiveTick`
  (params (DeltaSeconds :type "Float (single-precision)"))
  (bind _playerrootcomponent (`self.PlayerRootComponent`))
  (bind _overlappingactors (`PrimitiveComponent.GetOverlappingActors` (`self.TriggerBox`) null))
  (bind _output (`|GetArrayItem` _overlappingactors))
  (bind _rootcomponent (`Actor.RootComponent` _output))
  (bind _returnvalue (`KismetMathLibrary.FindLookAtRotation` (`SceneComponent.K2_GetComponentLocation` (`self.DefaultSceneRoot`)) (`SceneComponent.K2_GetComponentLocation` _rootcomponent)))
  (bind (_returnvalue_x _returnvalue_y) (`KismetMathLibrary.BreakVector` (* (`KismetMathLibrary.GetForwardVector` _returnvalue) (`self.KnockbackPower`))))
  (if (`KismetArrayLibrary.Array_IsEmpty` _overlappingactors)
    _
    (elif (`KismetSystemLibrary.IsValid` _output)
      (if (`KismetSystemLibrary.IsValid` _playerrootcomponent)
        (if (not (== _rootcomponent _playerrootcomponent))
          (bind _asbp_my_player_character (cast `/Game/TopDown/Blueprints/BP_MyPlayerCharacter` _output :!label _label)
            (:`then`
              (`self.K2_SetActorRotation` _returnvalue)
              (`Character.LaunchCharacter` _asbp_my_player_character (`KismetMathLibrary.MakeVector` _returnvalue_x _returnvalue_y) true true)
              (`/Game/TopDown/Blueprints/BP_MyPlayerCharacter.OnHit_OnServer` _asbp_my_player_character)
              (`self.K2_DestroyActor`))
            (:`CastFailed`
              (`self.K2_DestroyActor`))))
        (else
          (goto _label))))))

(fn `UserConstructionScript`)