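; Basic projectile that knocks back and damages player characters, and destroys itself after LifeSpanTime.
; The spawner passes its root component through an RPC event so the projectile can ignore it.
; Tick polls TriggerBox's first overlap, launches a hit character away and applies GE_BasicProjectileDamage through the Ability System.
; It calls OnDeath if the checked attribute reaches zero or below, and destroys itself on any non-owner hit.
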(event `self.ReceiveBeginPlay`
  (`KismetSystemLibrary.Delay` (`self.LifeSpanTime`))
  (`self.K2_DestroyActor`))

(event `RPC_PlayerRootComponent`
  (params (RootComponent :type "SceneComponent Object Reference (by ref)"))
  (set `self.PlayerRootComponent` RootComponent))

(event `self.PlayerSpawningRootComponent`
  (params (PlayerSpawningComponent :type "SceneComponent Object Reference"))
  (`self.RPC_PlayerRootComponent` PlayerSpawningComponent))

(event `self.ReceiveTick`
  (params (DeltaSeconds :type "Float (single-precision)"))
  (bind _playerrootcomponent (`self.PlayerRootComponent`))
  (bind _overlappingactors (`PrimitiveComponent.GetOverlappingActors` (`self.TriggerBox`) null))
  (bind _output (`|GetArrayItem` _overlappingactors))
  (bind _returnvalue (`AbilitySystemBlueprintLibrary.GetAbilitySystemComponent` _output))
  (bind _rootcomponent (`Actor.RootComponent` _output))
  (bind (_bsuccessfullyfoundattribute _returnvalue_2) (`AbilitySystemBlueprintLibrary.GetFloatAttributeFromAbilitySystemComponent` _returnvalue (struct :`AttributeName` "Health" :`Attribute` "/Script/FlareForge.MyCharacterAttributeSet:Health" :`AttributeOwner` "/Script/CoreUObject.Class'/Script/FlareForge.MyCharacterAttributeSet'")))
  (bind _returnvalue_3 (`KismetMathLibrary.FindLookAtRotation` (`SceneComponent.K2_GetComponentLocation` (`self.DefaultSceneRoot`)) (`SceneComponent.K2_GetComponentLocation` _rootcomponent)))
  (if (`KismetArrayLibrary.Array_IsEmpty` _overlappingactors)
    _
    (elif (`KismetSystemLibrary.IsValid` _output)
      (if (`KismetSystemLibrary.IsValid` _playerrootcomponent)
        (if (not (== _rootcomponent _playerrootcomponent))
          (bind _asbp_my_player_character (cast `/Game/TopDown/Blueprints/BP_MyPlayerCharacter` _output)
            (:`then`
              (`self.K2_SetActorRotation` _returnvalue_3)
              (`Character.LaunchCharacter` _asbp_my_player_character (* (`KismetMathLibrary.GetForwardVector` _returnvalue_3) (`self.KnockbackPower`)) true true)
              (`AbilitySystemComponent.BP_ApplyGameplayEffectToSelf` :`self` _returnvalue :`GameplayEffectClass` "/Game/Blueprints/GameplayEffects/Damage/GE_BasicProjectileDamage.GE_BasicProjectileDamage_C")
              (if _bsuccessfullyfoundattribute
                (if (<= _returnvalue_2 0.0)
                  (`/Game/TopDown/Blueprints/BP_MyPlayerCharacter.OnDeath` _asbp_my_player_character)
                  (`self.K2_DestroyActor`)
                  (else
                    (`self.K2_DestroyActor`)))
                (else
                  (`self.K2_DestroyActor`))))
            (:`CastFailed`
              (`self.K2_DestroyActor`))))))))

(fn `UserConstructionScript`)