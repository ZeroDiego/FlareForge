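; Temporary shield actor for the FightMe mechanic that destroys itself after ActiveTimer or on its first valid hit.
; It receives the spawning player's component through a multicast event and resolves that component's owner as the player character.
; Any capsule overlap calls that player's server buff, triggers the NPC-hit event on basic or homing strike projectiles, then destroys the shield.
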(event `self.ReceiveBeginPlay`
  (`KismetSystemLibrary.Delay` (`self.ActiveTimer`))
  (`self.K2_DestroyActor`))

(event `self.GetFightMePlayerReference`
  (params (PlayerSpawningRootComponent :type "SceneComponent Object Reference"))
  (`self.GetFightMePlayerReferenceMulticast` PlayerSpawningRootComponent))

(event `GetFightMePlayerReferenceOnServer`
  (params (PlayerRef :type "SceneComponent Object Reference")))

(event `GetFightMePlayerReferenceMulticast`
  (params (PlayerRef :type "SceneComponent Object Reference"))
  (set `self.Player Ref` PlayerRef))

(event `self.CapsuleComponent.OnComponentBeginOverlap`
  (params (OverlappedComponent :type "PrimitiveComponent Object Reference") (OtherActor :type "Actor Object Reference") (OtherComp :type "PrimitiveComponent Object Reference") (OtherBodyIndex :type Integer) (bFromSweep :type Boolean) (SweepResult :type "HitResult Structure (by ref)"))
  (`KismetSystemLibrary.PrintString` "hit")
  (bind _asbp_my_player_character (cast `/Game/TopDown/Blueprints/BP_MyPlayerCharacter` (`ActorComponent.GetOwner` (`self.Player Ref`))))
  (`/Game/TopDown/Blueprints/BP_MyPlayerCharacter.FightMeBuffCharacter_OnServer` _asbp_my_player_character)
  (bind _asbp_basic_projecitle (cast `/Game/Blueprints/Projectiles/BP_BasicProjecitle` OtherActor)
    (:`then`
      (`/Game/Blueprints/Projectiles/BP_BasicProjecitle.OnNPC_Hit_OnServer` _asbp_basic_projecitle))
    (:`CastFailed`
      _))
  (bind _asbp_homing_strike_projectile (cast `/Game/Blueprints/Projectiles/BP_HomingStrikeProjectile` OtherActor)
    (:`then`
      (`/Game/Blueprints/Projectiles/BP_HomingStrikeProjectile.OnNPC_Hit_OnServer` _asbp_homing_strike_projectile))
    (:`CastFailed`
      _))
  (`self.K2_DestroyActor`))

(fn `UserConstructionScript`)