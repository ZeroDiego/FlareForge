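; BP_Zone is a shrinking play zone that tracks whether player characters are outside it.
; On BeginPlay the server triggers one shrink, setting TargetSize to the zone mesh's X scale minus a fixed step, clamped.
; Tick interpolates the mesh's X and Y scale toward that target, leaving height unchanged.
; Begin and end overlaps set OutSideZone on BP_MyPlayerCharacter with authority only, skipping dead players on exit.
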(event `self.ReceiveBeginPlay`
  (bind _returnvalue_x (`KismetMathLibrary.BreakVector` (`SceneComponent.K2_GetComponentScale` (`self.SM_Zone`))))
  (`/Engine/EditorBlueprintResources/ActorMacros.Switch Has Authority`
    (:`Authority`
      (set `self.TargetSize` _returnvalue_x)
      (`self.Shrink On Server`))))

(event `Shrink On Server`
  (`self.Shrink`))

(event `Shrink`
  (bind _returnvalue_x (`KismetMathLibrary.BreakVector` (`SceneComponent.K2_GetComponentScale` (`self.SM_Zone`))))
  (set `self.TargetSize` (`KismetMathLibrary.FClamp` (- _returnvalue_x 99.0) 0.0 100.0)))

(event `self.ReceiveTick`
  (params (DeltaSeconds :type "Float (single-precision)"))
  (bind (_returnvalue_x _returnvalue_y _returnvalue_z) (`KismetMathLibrary.BreakVector` (`SceneComponent.K2_GetComponentScale` (`self.SM_Zone`))))
  (bind _returnvalue (`KismetMathLibrary.FInterpTo` _returnvalue_x (`self.TargetSize`) DeltaSeconds (`self.ZoneShrinkSpeed`)))
  ;[1 1 1] Current scale for Zone
  (if (not (== _returnvalue_x 0.0))
    (`SceneComponent.SetWorldScale3D` (`self.SM_Zone`) (`KismetMathLibrary.MakeVector` _returnvalue _returnvalue _returnvalue_z))))

(event `self.ReceiveActorBeginOverlap`
  (params (OtherActor :type "Actor Object Reference"))
  ;[1 1 1] Overlap with player
  (`self.Handle_Zone_Logic` OtherActor))

(event `self.ReceiveActorEndOverlap`
  (params (OtherActor :type "Actor Object Reference"))
  ;[1 1 1] Overlap with player
  (bind _asbp_my_player_character (cast `/Game/TopDown/Blueprints/BP_MyPlayerCharacter` OtherActor))
  (if (not (`/Game/TopDown/Blueprints/BP_MyPlayerCharacter.bDead` _asbp_my_player_character))
    (`self.Handle_Zone_Logic` _asbp_my_player_character true)))

(fn `Handle_Zone_Logic`
  (params (Actor :type "Object Object Reference") (bOutSideZone :type Boolean))
  (`/Engine/EditorBlueprintResources/ActorMacros.Switch Has Authority`
    (:`Authority`
      (if (== (`GameplayStatics.GetObjectClass` Actor) "/Game/TopDown/Blueprints/BP_MyPlayerCharacter.BP_MyPlayerCharacter_C")
        (bind _asbp_my_player_character (cast `/Game/TopDown/Blueprints/BP_MyPlayerCharacter` Actor))
        (set `/Game/TopDown/Blueprints/BP_MyPlayerCharacter.bOutSideZone` bOutSideZone _asbp_my_player_character)))))

(fn `UserConstructionScript`)