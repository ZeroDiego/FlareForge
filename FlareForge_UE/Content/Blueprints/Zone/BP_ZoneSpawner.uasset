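; BP_ZoneSpawner is a one-shot actor that places a BP_Zone at a random spot once multiple player characters are in the level.
; Tick polls for BP_MyPlayerCharacter actors until more than one exists, then fires SpawnZoneOnServer once, which calls SpawnZone.
; SpawnZone sizes the Box by RandomPositionBoxSize, spawns the zone at a random XY inside it with a fixed Z, then destroys the spawner.
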(event `Spawn Zone on Server`
  (`self.Spawn Zone`))

(event `self.ReceiveBeginPlay`)

(event `self.ReceiveTick`
  (params (DeltaSeconds :type "Float (single-precision)"))
  ;[1 1 1] Count Amount of players
  (if (not (`self.bAllCharactersAreIn`))
    (bind _outactors (`GameplayStatics.GetAllActorsOfClass` "/Game/TopDown/Blueprints/BP_MyPlayerCharacter.BP_MyPlayerCharacter_C"))
    (if (> (`KismetArrayLibrary.Array_Length` _outactors) 1)
      (`/Engine/EditorBlueprintResources/StandardMacros.DoOnce` false
        (:`Completed`
          (set `self.bAllCharactersAreIn` true)
          (`self.Spawn Zone on Server`))))))

(event `Spawn Zone`
  (bind _box (`self.Box`))
  (bind _randompositionboxsize (`self.RandomPositionBoxSize`))
  (bind (_returnvalue_x _returnvalue_y) (`KismetMathLibrary.BreakVector` (`KismetMathLibrary.RandomPointInBoundingBox` (`SceneComponent.K2_GetComponentLocation` _box) (`BoxComponent.GetUnscaledBoxExtent` _box))))
  (`BoxComponent.SetBoxExtent` (`self.Box`) (`KismetMathLibrary.MakeVector` _randompositionboxsize _randompositionboxsize) true)
  (`|SpawnActorFromClass` "/Game/Blueprints/Zone/BP_Zone.BP_Zone_C" (`KismetMathLibrary.MakeTransform` (`KismetMathLibrary.MakeVector` _returnvalue_x _returnvalue_y -50.0)) "Undefined" "MultiplyWithRoot" null null)
  (`self.K2_DestroyActor`))

(fn `UserConstructionScript`)