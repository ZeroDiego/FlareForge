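; Homing projectile that knocks back top-down characters on overlap and destroys itself on impact or when its lifespan ends.
; Lock-on requests go through an RPC that sets the projectile movement's homing target, excluding the spawning player's root component, and re-runs after a delay with a newly found target to keep switching.
; The trigger box ignores the spawner, turns toward the hit character and launches it away with knockback power.
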(event `self.ReceiveBeginPlay`
  (`KismetSystemLibrary.Delay` (`self.LifeSpanTime`))
  (`self.K2_DestroyActor`))

(event `RPC_LockOn`
  (params (TargetComponent :type "SceneComponent Object Reference (by ref)") (PlayerSpawningRootComponent :type "SceneComponent Object Reference (by ref)"))
  (bind _projectilemovement (`self.ProjectileMovement`))
  (set `self.PlayerSpawningReference` PlayerSpawningRootComponent)
  (if (not (== TargetComponent PlayerSpawningRootComponent))
    (set `ProjectileMovementComponent.HomingTargetComponent` TargetComponent _projectilemovement)
    (set `ProjectileMovementComponent.bIsHomingProjectile` true _projectilemovement))
  (`KismetSystemLibrary.Delay` (`self.TargetSwitchTime`))
  (`self.RPC_LockOn` (`self.FindHomingStrikeTarget`) PlayerSpawningRootComponent))

(event `self.LockOn`
  (params (TargetComponent :type "SceneComponent Object Reference") (PlayerSpawningRootComponent :type "SceneComponent Object Reference"))
  (`self.RPC_LockOn` TargetComponent PlayerSpawningRootComponent))

(event `self.TriggerBox.OnComponentBeginOverlap`
  (params (OverlappedComponent :type "PrimitiveComponent Object Reference") (OtherActor :type "Actor Object Reference") (OtherComp :type "PrimitiveComponent Object Reference") (OtherBodyIndex :type Integer) (bFromSweep :type Boolean) (SweepResult :type "HitResult Structure (by ref)"))
  (bind _playerspawningreference (`self.PlayerSpawningReference`))
  (bind _rootcomponent (`Actor.RootComponent` OtherActor))
  (bind _returnvalue (`KismetMathLibrary.FindLookAtRotation` (`SceneComponent.K2_GetComponentLocation` (`self.DefaultSceneRoot`)) (`SceneComponent.K2_GetComponentLocation` _rootcomponent)))
  (if (`KismetSystemLibrary.IsValid` _playerspawningreference)
    (if (not (== _rootcomponent _playerspawningreference))
      (bind _asbp_top_down_character (cast `/Game/TopDown/Blueprints/BP_TopDownCharacter` OtherActor))
      (`self.K2_SetActorRotation` _returnvalue)
      (`Character.LaunchCharacter` _asbp_top_down_character (* (`KismetMathLibrary.GetForwardVector` _returnvalue) (`self.KnockbackPower`)) true true)
      (`self.K2_DestroyActor`))))

(fn `UserConstructionScript`)