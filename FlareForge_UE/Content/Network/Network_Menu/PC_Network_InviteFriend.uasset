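; Player controller for the invite-friend network menu, which opens the lobby UI and registers the player's lobby info with the game mode.
; On BeginPlay, SetUp gives local controllers the lobby widget, cursor and game-and-UI input, then calls SetPlayerNameOnServer with an empty name.
; That event stores the name and calls UpdatePlayerLobbyInfo on GM_Network_InviteFriend; a separate event repeats the update after a short delay.
; An older InviteFriendUI creation chain is left disconnected.
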(event `TryAgainUpdataingLobbyInfo`
  (`KismetSystemLibrary.Delay` 0.1)
  (bind _asgm_network_invite_friend (cast `/Game/Network/Network_Menu/GM_Network_InviteFriend` (`GameplayStatics.GetGameMode`)))
  (`/Game/Network/Network_Menu/GM_Network_InviteFriend.UpdatePlayerLobbyInfo` _asgm_network_invite_friend self))

(event `SetPlayerNameOnServer`
  (params (PlayerName :type Text))
  (setmembers `/Game/Network/Network_Lobby/S_PlayerLobbyInfo` :`StructRef` (`self.PlayerLobbyInfo`) :`PlayerName` PlayerName)
  (bind _asgm_network_invite_friend (cast `/Game/Network/Network_Menu/GM_Network_InviteFriend` (`GameplayStatics.GetGameMode`)))
  (`/Game/Network/Network_Menu/GM_Network_InviteFriend.UpdatePlayerLobbyInfo` _asgm_network_invite_friend self))

(event `self.ReceiveBeginPlay`
  (`self.SetUp`))

(fn `SetUp`
  (if (`self.IsLocalPlayerController`)
    (set `self.bShowMouseCursor` true)
    (`WidgetBlueprintLibrary.SetInputMode_GameAndUIEx` self null)
    (bind _returnvalue (`|CreateWidget` "/Game/Network/Network_Lobby/WBP_LobbyUI.WBP_LobbyUI_C"))
    (bind _output_get (set `self.LobbyUIRef` _returnvalue))
    (`UserWidget.AddToViewport` _output_get 0)
    (`self.SetPlayerNameOnServer` "")))

(fn `UserConstructionScript`)